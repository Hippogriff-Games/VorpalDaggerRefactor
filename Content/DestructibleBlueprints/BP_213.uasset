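; BP_213 is a destructible prop that reduces score and switches narration when a permitted actor hits its static mesh.
; On hit, CheckDeathAllowed gates ScoreReduction, then each BP_NarrationManager tagged "Narration" receives ChangeSequence with the game mode's current narration player.
; It creates an auto-playing Narration sequence player after that call, although the call takes that player's actor as the new sequence.
; The mesh component is destroyed immediately and the actor after a short delay.
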(event OnComponentHit(StaticMesh)
  (params (HitComponent :type Primitive%20Component%20Object%20Reference) (OtherActor :type Actor%20Object%20Reference) (OtherComp :type Primitive%20Component%20Object%20Reference) (NormalImpulse :type Vector :default "0, 0, 0") (Hit :type Hit%20Result%20Structure%20%28by%20ref%29))
  (bind _cankill (CallFunction|CheckDeathAllowed OtherActor))
  (if _cankill
    (CallFunction|ScoreReduction)
    (bind _outactors (Actor|GetAllActorswithTag "Narration"))
    (for _array_element _outactors
      (bind _asbp_narration_manager (Utilities|Casting|CastToBP_NarrationManager _array_element))
      (bind _asgm_vorpal_dagger (Utilities|Casting|CastToGM_VorpalDagger (Game|GetGameMode)))
      (Default|ChangeSequence _asbp_narration_manager (Variables|/Game/ThirdPersonBP/Blueprints/GM_VorpalDagger.GM_VorpalDagger_C|GetCurrentNarrationPlayer _asgm_vorpal_dagger) (stale _outactor))
      (bind _outactor (Sequencer|Player|CreateLevelSequencePlayer (Variables|Default|Getnarration) (Utilities|Struct|MakeMovieSceneSequencePlaybackSettings true "(Value=0)" 1.0 0.0 false false false false false false false false)))
      (Components|DestroyComponent (Variables|Default|GetStaticMesh))
      (Utilities|FlowControl|Delay 3.0)
      (Actor|DestroyActor))))

(fn ConstructionScript)