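; BP_Destructible is a breakable prop that shatters on impact and costs the player points.
; A mesh hit breaks it if its own speed exceeds MinVelocity or the other actor is a BP_VorpalDaggerController, while hits from other destructibles are ignored.
; Breaking decreases GM_VorpalDagger's score once by PointValue, hides the mesh and disables its collision.
; It spawns BP_Piece debris with random materials from the mesh, plays a sound, then destroys itself.
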(event OnComponentHit(StaticMesh)
  (params (HitComponent :type Primitive%20Component%20Object%20Reference) (OtherActor :type Actor%20Object%20Reference) (OtherComp :type Primitive%20Component%20Object%20Reference) (NormalImpulse :type Vector :default "0, 0, 0") (Hit :type Hit%20Result%20Structure%20%28by%20ref%29))
  (bind _cankill (CallFunction|CheckDeathAllowed OtherActor))
  (if _cankill
    (CallFunction|ScoreReduction)
    (CallFunction|Die)))

(event Custom|Die
  (Collision|SetCollisionEnabled (Variables|Default|GetStaticMesh) "NoCollision")
  (Rendering|SetVisibility (Variables|Default|GetStaticMesh) false true)
  (for _index (range 0 (Variables|Default|GetPieces))
    (bind _returnvalue (Game|SpawnActorfromClass "/Game/ThirdPersonBP/Blueprints/BP_Piece.BP_Piece_C" (Transformation|GetActorTransform) "AdjustIfPossibleButAlwaysSpawn" self 0))
    (Rendering|Material|SetMaterial (Variables|/Game/ThirdPersonBP/Blueprints/BP_Piece.BP_Piece_C|GetPiece _returnvalue) 0 (Rendering|Material|GetMaterial (Variables|Default|GetStaticMesh) (Math|Random|RandomInteger (Utilities|Array|Length (Rendering|Material|GetMaterials (Variables|Default|GetStaticMesh)))))))
  (Audio|PlaySoundatLocation "/Game/Audio/SoundEffects/Break_Cue.Break_Cue" (Transformation|GetActorLocation self) "0, 0, 0" 1.0 1.0 0.0 0 0 0)
  (Utilities|FlowControl|Delay 0.2)
  (Actor|DestroyActor))

(event EventBeginPlay)

(event Collision|EventActorBeginOverlap
  (params (OtherActor :type Actor%20Object%20Reference)))

(event EventTick
  (params (DeltaSeconds :type Float%20%28single-precision%29)))

(fn ConstructionScript)

(fn CheckDeathAllowed
  (params (Object :type Object%20Object%20Reference))
  (Utilities|Casting|CastToBP_Destructible Object
    (:CastFailed
      (if (> (Math|Vector|VectorLength (Transformation|GetComponentVelocity (Variables|Default|GetStaticMesh))) (Variables|Default|GetMinVelocity))
        (return true)
        (else
          (Utilities|Casting|CastToBP_VorpalDaggerController Object
            (:then
              (return true))
            (:CastFailed
              (return false))))))))

(fn ScoreReduction
  (Utilities|FlowControl|DoOnce false
    (:Completed
      (bind _asgm_vorpal_dagger (Utilities|Casting|CastToGM_VorpalDagger (Game|GetGameMode)))
      (Default|DecreaseScore _asgm_vorpal_dagger (Variables|Default|Getpoint%20value))
      (return))))