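; Base NPC character that gets decapitated when its capsule is hit by the vorpal dagger controller.
; The hit hides the head bone, spawns neck blood, removes the capsule and triggers Death1.
; Death1 ragdolls the mesh, updates the tagged narration manager, plays the Narration level sequence, then destroys the actor after a delay.
; Helper functions expose the patrol route and map movement states to walk speeds.
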(event OnComponentHit(CapsuleComponent)
  (params (HitComponent :type Primitive%20Component%20Object%20Reference) (OtherActor :type Actor%20Object%20Reference) (OtherComp :type Primitive%20Component%20Object%20Reference) (NormalImpulse :type Vector :default "0, 0, 0") (Hit :type Hit%20Result%20Structure%20%28by%20ref%29))
  (bind _mesh (Variables|Character|GetMesh))
  (bind _asbp_vorpal_dagger_controller (Utilities|Casting|CastToBP_VorpalDaggerController OtherActor)
    (:then
      (Utilities|IsValid _asbp_vorpal_dagger_controller
        (:Is%20Valid
          (Components|SkinnedMesh|HideBonebyName (Variables|Character|GetMesh) "Head" "PBO_None")
          (Effects|SpawnEmitterAttached "/Game/Particles/P_Blood.P_Blood" _mesh "Neck" (Transformation|GetSocketLocation _mesh "Neck") "0, 0, 0" "1.000000,1.000000,1.000000" "KeepWorldPosition")
          (Components|DestroyComponent (Variables|Collision|GetCapsuleComponent))
          (CallFunction|Death1))
        (:Is%20Not%20Valid
          (Development|PrintString "Not valid"))))
    (:CastFailed
      (Development|PrintString "fuck everythin"))))

(event Custom|Death1
  (Physics|SetSimulatePhysics (Variables|Character|GetMesh) true)
  (bind _outactors (Actor|GetAllActorswithTag "Narration"))
  (for _array_element _outactors
    (bind _asbp_narration_manager (Utilities|Casting|CastToBP_NarrationManager _array_element))
    (bind _asgm_vorpal_dagger (Utilities|Casting|CastToGM_VorpalDagger (Game|GetGameMode)))
    (Default|ChangeSequence _asbp_narration_manager (Variables|/Game/ThirdPersonBP/Blueprints/GM_VorpalDagger.GM_VorpalDagger_C|GetCurrentNarrationPlayer _asgm_vorpal_dagger))
    (Sequencer|Player|CreateLevelSequencePlayer (Variables|Default|GetNarration) (Utilities|Struct|MakeMovieSceneSequencePlaybackSettings true "(Value=0)" 1.0 0.0 false false false false false false false false))
    (Pawn|Components|CharacterMovement|DisableMovement (Variables|Character|GetCharacterMovement))
    (Utilities|FlowControl|Delay 5.0)
    (Actor|DestroyActor)))

(event EventBeginPlay)

(fn ConstructionScript)

(fn GetPatrolRoute
  (return (Variables|AI|GetPatrolRoute)))

(fn SetMovementSpeed
  (params (Speed :type E_MovementSpeed%20Enum :default "NewEnumerator0"))
  (bind _output_get (Variables|/Script/Engine.CharacterMovementComponent|SetMaxWalkSpeed (Variables|Character|GetCharacterMovement) (Utilities|Select :Index Speed :NewEnumerator0 0.0 :NewEnumerator1 1e+02 :NewEnumerator2 3e+02 :NewEnumerator3 5e+02)))
  (return _output_get))