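; End-of-game trigger that shows the results screen and plays an ending narration chosen by score.
; On overlap it disables its collision, switches input to UI only and fills WBP_End with the game mode's modified score and time.
; If the overlapping actor is BP_VorpalDaggerController, it calls ChangeSequence on tagged narration managers, then picks good, mild or bad ending by raw score.
; Duration-based delays chain each ending's level sequences before the trigger destroys itself.
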(event OnComponentBeginOverlap(CollisionComponent)
  (params (OverlappedComponent :type Primitive%20Component%20Object%20Reference) (OtherActor :type Actor%20Object%20Reference) (OtherComp :type Primitive%20Component%20Object%20Reference) (OtherBodyIndex :type Integer) (bFromSweep :type Boolean) (SweepResult :type Hit%20Result%20Structure%20%28by%20ref%29))
  (bind _returnvalue (Game|GetPlayerController 0))
  (Collision|SetCollisionEnabled (Variables|Default|GetCollisionComponent) "NoCollision")
  (Input|SetInputModeUIOnly _returnvalue 0 "DoNotLock")
  (bind _returnvalue_2 (UserInterface|CreateWidget "/Game/ThirdPersonBP/UI/WBP_End.WBP_End_C" _returnvalue))
  (UserInterface|Viewport|AddtoViewport _returnvalue_2 -1)
  (bind _asgm_vorpal_dagger (Utilities|Casting|CastToGM_VorpalDagger (Game|GetGameMode)))
  (bind _returnvalue_3 (Default|GetScorewithModifier _asgm_vorpal_dagger))
  (Rendering|Components|TextRender|SetText (Variables|/Game/ThirdPersonBP/UI/WBP_End.WBP_End_C|GetScoreSlot _returnvalue_2) (Utilities|Text|ToText(Integer) _returnvalue_3))
  (bind _seconds (Default|GetCurrentTime _asgm_vorpal_dagger))
  (Rendering|Components|TextRender|SetText (Variables|/Game/ThirdPersonBP/UI/WBP_End.WBP_End_C|GetTimeSlot _returnvalue_2) (Utilities|Text|ToText(String) (Class|KismetStringLibrary|TimeSecondstoString (Math|Conversions|ToFloat(Integer) _seconds))))
  (Utilities|Casting|CastToBP_VorpalDaggerController OtherActor)
  (bind _asgm_vorpal_dagger_2 (Utilities|Casting|CastToGM_VorpalDagger (Game|GetGameMode)))
  (bind _score (Default|GetScore _asgm_vorpal_dagger_2))
  (bind _outactors (Actor|GetAllActorswithTag "Narration"))
  (for _array_element _outactors
    (bind _asbp_narration_manager (Utilities|Casting|CastToBP_NarrationManager _array_element))
    (bind _asgm_vorpal_dagger_3 (Utilities|Casting|CastToGM_VorpalDagger (Game|GetGameMode)))
    (Default|ChangeSequence _asbp_narration_manager (Variables|/Game/ThirdPersonBP/Blueprints/GM_VorpalDagger.GM_VorpalDagger_C|GetCurrentNarrationPlayer _asgm_vorpal_dagger_3))
    (if (== _score 1000)
      (bind _outactor (Sequencer|Player|CreateLevelSequencePlayer "/Game/Audio/Voiceover/SubtitleStuff/NLS_stuff/NLS_GoodEndingPart1.NLS_GoodEndingPart1" (Utilities|Struct|MakeMovieSceneSequencePlaybackSettings true "(Value=0)" 1.0 0.0 false false false false false false false false)))
      (Utilities|FlowControl|Delay (Class|TimeManagementBlueprintLibrary|ToSeconds(QualifiedFrameTime) (Media|MediaPlayer|GetDuration (Variables|/Script/LevelSequence.LevelSequenceActor|GetSequencePlayer _outactor))))
      (bind _outactor_2 (Sequencer|Player|CreateLevelSequencePlayer "/Game/Audio/Voiceover/SubtitleStuff/NLS_stuff/NLS_GoodEndingPart2.NLS_GoodEndingPart2" (Utilities|Struct|MakeMovieSceneSequencePlaybackSettings true "(Value=0)" 1.0 0.0 false false false false false false false false)))
      (Utilities|FlowControl|Delay (Class|TimeManagementBlueprintLibrary|ToSeconds(QualifiedFrameTime) (Media|MediaPlayer|GetDuration (Variables|/Script/LevelSequence.LevelSequenceActor|GetSequencePlayer _outactor_2))))
      (Actor|DestroyActor)
      (elif (and (>= _score 1) (< _score 1000))
        (bind _outactor_3 (Sequencer|Player|CreateLevelSequencePlayer "/Game/Audio/Voiceover/SubtitleStuff/NLS_stuff/NLS_MildEndingPart1.NLS_MildEndingPart1" (Utilities|Struct|MakeMovieSceneSequencePlaybackSettings true "(Value=0)" 1.0 0.0 false false false false false false false false)))
        (Utilities|FlowControl|Delay (Class|TimeManagementBlueprintLibrary|ToSeconds(QualifiedFrameTime) (Media|MediaPlayer|GetDuration (Variables|/Script/LevelSequence.LevelSequenceActor|GetSequencePlayer _outactor_3))))
        (bind _outactor_4 (Sequencer|Player|CreateLevelSequencePlayer "/Game/Audio/Voiceover/SubtitleStuff/NLS_stuff/NLS_MildEndingPart2.NLS_MildEndingPart2" (Utilities|Struct|MakeMovieSceneSequencePlaybackSettings true "(Value=0)" 1.0 0.0 false false false false false false false false)))
        (Utilities|FlowControl|Delay (Class|TimeManagementBlueprintLibrary|ToSeconds(QualifiedFrameTime) (Media|MediaPlayer|GetDuration (Variables|/Script/LevelSequence.LevelSequenceActor|GetSequencePlayer _outactor_4))))
        (Actor|DestroyActor)
        (else
          (bind _outactor_5 (Sequencer|Player|CreateLevelSequencePlayer "/Game/Audio/Voiceover/SubtitleStuff/NLS_stuff/NLS_BadEndingPart1.NLS_BadEndingPart1" (Utilities|Struct|MakeMovieSceneSequencePlaybackSettings true "(Value=0)" 1.0 0.0 false false false false false false false false)))
          (Utilities|FlowControl|Delay (Class|TimeManagementBlueprintLibrary|ToSeconds(QualifiedFrameTime) (Media|MediaPlayer|GetDuration (Variables|/Script/LevelSequence.LevelSequenceActor|GetSequencePlayer _outactor_5))))
          (bind _outactor_6 (Sequencer|Player|CreateLevelSequencePlayer "/Game/Audio/Voiceover/SubtitleStuff/NLS_stuff/NLS_BadEndingPart2.NLS_BadEndingPart2" (Utilities|Struct|MakeMovieSceneSequencePlaybackSettings true "(Value=0)" 1.0 0.0 false false false false false false false false)))
          (Utilities|FlowControl|Delay (Class|TimeManagementBlueprintLibrary|ToSeconds(QualifiedFrameTime) (Media|MediaPlayer|GetDuration (Variables|/Script/LevelSequence.LevelSequenceActor|GetSequencePlayer _outactor_6))))
          (bind _outactor_7 (Sequencer|Player|CreateLevelSequencePlayer "/Game/Audio/Voiceover/SubtitleStuff/NLS_stuff/NLS_BadEndingPart3.NLS_BadEndingPart3" (Utilities|Struct|MakeMovieSceneSequencePlaybackSettings true "(Value=0)" 1.0 0.0 false false false false false false false false)))
          (Utilities|FlowControl|Delay (Class|TimeManagementBlueprintLibrary|ToSeconds(QualifiedFrameTime) (Media|MediaPlayer|GetDuration (Variables|/Script/LevelSequence.LevelSequenceActor|GetSequencePlayer _outactor_7))))
          (Actor|DestroyActor))))))

(fn ConstructionScript
  (|CallParentFunction))